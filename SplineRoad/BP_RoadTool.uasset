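; Spline road tool that procedurally builds a road, optional light poles and debug point numbers in its Construction Script.
; BuildRoad chains spline meshes at fixed spacing, stretching the last to the spline end, with optional roll and query collision.
; All segments share one dynamic material instance driving traffic direction, speed and tiling.
; BuildPoles spawns child actors along the spline, alternating sides via right-vector offset and flipped yaw.
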(event `self.ReceiveBeginPlay`)

(fn `Build_Poles`
  (bind _spacing_lightpoles (`self.Spacing_LightPoles`))
  (bind _spline (`self.Spline`))
  (for _index (range (`.ReturnValue` (`KismetMathLibrary.FMod` (`SplineComponent.GetSplineLength` (`self.Spline`)) _spacing_lightpoles)))
    (bind _returnvalue (* _index _spacing_lightpoles))
    (bind _returnvalue_2 (`SplineComponent.GetRightVectorAtDistanceAlongSpline` _spline _returnvalue "Local"))
    (bind _returnvalue_3 (* _returnvalue_2 (`self.CenterOffset_LightPoles`)))
    (bind _returnvalue_4 (!= (mod _index 2) 0))
    (bind (_returnvalue_roll _returnvalue_pitch _returnvalue_yaw) (`KismetMathLibrary.BreakRotator` (`KismetMathLibrary.MakeRotFromZ` _returnvalue_2)))
    (`AddComponent|NODE_AddChildActorComponent-0` :`RelativeTransform` (`KismetMathLibrary.MakeTransform` (+ (`SplineComponent.GetLocationAtDistanceAlongSpline` _spline _returnvalue "Local") (select `bool` _returnvalue_4 :`false` _returnvalue_3 :`true` (* _returnvalue_3 -1))) (`KismetMathLibrary.MakeRotator` 0.0 0.0 (+ _returnvalue_yaw (`KismetMathLibrary.SelectFloat` 180.0 0.0 _returnvalue_4)))))))

(fn `Build_Road`
  (locals (LocalStartLocation :type "Vector Structure") (LocalEndLocation :type "Vector Structure") (LocalStartTangent :type "Vector Structure") (LocalEndTangent :type "Vector Structure") (LocalCurrentSplineMesh :type "SplineMeshComponent Object Reference") (LocalCurrentLoopIndex :type Integer) (Local_Road_MID :type "MaterialInstanceDynamic Object Reference"))
  (bind _localcurrentsplinemesh (`local.LocalCurrentSplineMesh`))
  (bind _returnvalue (`KismetMathLibrary.MakeVector2D` (`self.Width_Road`) 1.0))
  (bind _returnvalue_2 (`SplineComponent.GetSplineLength` (`self.Spline`)))
  (bind _returnvalue_3 (* (`local.LocalCurrentLoopIndex`) (`self.Spacing_Road`)))
  (bind _returnvalue_4 (+ (`local.LocalCurrentLoopIndex`) 1))
  (bind (_returnvalue_x _returnvalue_y _returnvalue_z) (`KismetMathLibrary.BreakVector` (`SplineComponent.GetRightVectorAtDistanceAlongSpline` (`self.Spline`) _returnvalue_3 "Local")))
  (bind (_remainder _returnvalue_5) (`KismetMathLibrary.FMod` _returnvalue_2 (`self.Spacing_Road`)))
  (bind _returnvalue_6 (* _returnvalue_4 (`KismetMathLibrary.SelectFloat` _returnvalue_2 (`self.Spacing_Road`) (== _returnvalue_5 _returnvalue_4))))
  (bind (_returnvalue_x_2 _returnvalue_y_2 _returnvalue_z_2) (`KismetMathLibrary.BreakVector` (`SplineComponent.GetRightVectorAtDistanceAlongSpline` (`self.Spline`) _returnvalue_6 "Local")))
  (`|ExecutionSequence`
    (:`then_0`
      ;[1 1 1] Create and store Material Instance of MI_Road_Lighting
      (bind _returnvalue_7 (`KismetMaterialLibrary.CreateDynamicMaterialInstance` (`self.Road_Material`)))
      (set `local.Local_Road_MID` _returnvalue_7)
      ;[1 1 1] Traffic Material Settings
      (`MaterialInstanceDynamic.SetScalarParameterValue` (`local.Local_Road_MID`) "ReverseTrafficDirection?" (select `bool` (`self.Reverse_Traffic?`) :`true` 1.0))
      (`MaterialInstanceDynamic.SetScalarParameterValue` (`local.Local_Road_MID`) "OneWayTraffic?" (select `bool` (`self.OneWay_Traffic?`) :`true` 1.0))
      (`MaterialInstanceDynamic.SetScalarParameterValue` (`local.Local_Road_MID`) "Traffic_Speed_01" (`self.Traffic_Speed_01`))
      (`MaterialInstanceDynamic.SetScalarParameterValue` (`local.Local_Road_MID`) "Traffic_Speed_02" (`self.Traffic_Speed_02`))
      (`MaterialInstanceDynamic.SetScalarParameterValue` (`local.Local_Road_MID`) "Tiling_Traffic_U" (`KismetMathLibrary.Conv_IntToDouble` (`self.Tiling_Traffic_U`))))
    (:`then_1`
      ;[1 0 0] For Loop!
      (for _index (range _returnvalue_5)
        (set `local.LocalCurrentLoopIndex` _index)
        (set `local.LocalStartLocation` (`SplineComponent.GetLocationAtDistanceAlongSpline` (`self.Spline`) _returnvalue_3 "Local"))
        (set `local.LocalStartTangent` (* (`SplineComponent.GetDirectionAtDistanceAlongSpline` (`self.Spline`) _returnvalue_3 "Local") (`self.Spacing_Road`)))
        (set `local.LocalEndLocation` (`SplineComponent.GetLocationAtDistanceAlongSpline` (`self.Spline`) _returnvalue_6 "Local"))
        (set `local.LocalEndTangent` (* (`SplineComponent.GetDirectionAtDistanceAlongSpline` (`self.Spline`) _returnvalue_6 "Local") (`self.Spacing_Road`)))
        (`|ExecutionSequence`
          (:`then_0`
            (bind _returnvalue_8 (`AddComponent|NODE_AddSplineMeshComponent-2`))
            (bind _output_get (set `local.LocalCurrentSplineMesh` _returnvalue_8))
            (`StaticMeshComponent.SetStaticMesh` _output_get (`self.RoadMesh`))
            (`SplineMeshComponent.SetStartAndEnd` _localcurrentsplinemesh (`local.LocalStartLocation`) (`local.LocalStartTangent`) (`local.LocalEndLocation`) (`local.LocalEndTangent`) true)
            (`SplineMeshComponent.SetStartScale` _localcurrentsplinemesh _returnvalue true)
            (`SplineMeshComponent.SetEndScale` _localcurrentsplinemesh _returnvalue true)
            (`PrimitiveComponent.SetMaterial` (`local.LocalCurrentSplineMesh`) 0 (`local.Local_Road_MID`)))
          (:`then_1`
            (if (`self.Apply_Roll?`)
              (`SplineMeshComponent.SetStartRoll` (`local.LocalCurrentSplineMesh`) _returnvalue_z true)
              (`SplineMeshComponent.SetEndRoll` (`local.LocalCurrentSplineMesh`) _returnvalue_z_2 true)))
          (:`then_2`
            (`PrimitiveComponent.SetCollisionEnabled` (`local.LocalCurrentSplineMesh`) (select `bool` (`self.Collision_Road?`) :`false` "NoCollision" :`true` "QueryOnly" :!type "ECollisionEnabled Enum"))))))))

(fn `UserConstructionScript`
  (bind _spline (`self.Spline`))
  (`|ExecutionSequence`
    (:`then_0`
      (`self.Build_Road`))
    (:`then_1`
      (if (`self.Build_LightPoles?`)
        (`self.Build_Poles`)))
    (:`then_2`
      (for _index (range (`SplineComponent.GetNumberOfSplinePoints` (`self.Spline`)))
        ;[1 1 1] Draw Spline Point Numbers
        (if (`self.DrawSplinePointNumbers?`)
          (bind (_returnvalue_x _returnvalue_y _returnvalue_z) (`KismetMathLibrary.BreakVector` (`SplineComponent.GetLocationAtSplinePoint` _spline _index "Local")))
          (bind _returnvalue (`AddComponent|NODE_AddTextRenderComponent-0` :`RelativeTransform` (`KismetMathLibrary.MakeTransform` (`KismetMathLibrary.MakeVector` _returnvalue_x _returnvalue_y (+ _returnvalue_z 500.0)) (`SplineComponent.GetRotationAtSplinePoint` _spline _index "Local") (3.0 3.0 3.0))))
          (`TextRenderComponent.K2_SetText` _returnvalue (`KismetTextLibrary.Conv_IntToText` _index)))))))